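; Isometric camera pawn for a tower defence game, with a spring arm and camera.
; On BeginPlay it adds the isometric camera Enhanced Input mapping context to its player controller.
; The move action feeds movement input along the actor's forward vector only, using the Y axis.
; When the game mode's debug flag is on, Tick draws the spring arm line and a cone at the camera.
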(event `self.ReceiveTick`
  (params (DeltaSeconds :type "Float (single-precision)"))
  (bind _springarm (`self.SpringArm`))
  (bind _returnvalue (`SceneComponent.K2_GetComponentLocation` _springarm))
  (bind _asbp_tower_defence_game_mode (cast `/Game/GameMode/BP_TowerDefenceGameMode` (`GameplayStatics.GetGameMode`)))
  (if (`/Game/GameMode/BP_TowerDefenceGameMode.DebugMode` _asbp_tower_defence_game_mode)
    (`KismetSystemLibrary.DrawDebugLine` _returnvalue (+ _returnvalue (* (`KismetMathLibrary.NegateVector` (`SceneComponent.GetForwardVector` _springarm)) (`SpringArmComponent.TargetArmLength` _springarm))) (struct :`R` 0.916582 :`G` 0.125837 :`B` 1.0 :`A` 1.0) 0.0 1.0)
    (`KismetSystemLibrary.DrawDebugConeInDegrees` (`SceneComponent.K2_GetComponentLocation` (`self.Camera`)))))

(event `self.ReceiveBeginPlay`
  ; Settup Mapping
  (bind _asplayer_controller (cast `PlayerController` (`self.GetController`)))
  (bind _returnvalue (pcsubsystem `EnhancedInputLocalPlayerSubsystem` _asplayer_controller))
  (`/Engine/EditorBlueprintResources/StandardMacros.IsValid` _returnvalue
    (:`Is Valid`
      (message `EnhancedInputSubsystemInterface.AddMappingContext` _returnvalue "/Game/Controller/IsometricCameraMapping.IsometricCameraMapping" 0 (struct)))))

(event `EnhancedInput|/Game/Actions/IA_Move`
  (params (ActionValue :type "Vector2D Structure") (ElapsedSeconds :type "Float (double-precision)") (TriggeredSeconds :type "Float (double-precision)") (InputAction :type "InputAction Object Reference" :default "/Game/Actions/IA_Move.IA_Move"))
  ; Movement
  (:`Triggered`
    (`self.AddMovementInput` (`self.GetActorForwardVector`) ActionValue_Y)))

(fn `UserConstructionScript`)